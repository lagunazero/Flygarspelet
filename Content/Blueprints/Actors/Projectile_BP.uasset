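; Projectile actor that damages what it hits or overlaps, then destroys itself and spawns an explosion particle effect.
; Hit and overlap events both feed DamageObject, which skips actors sharing the projectile's instigator controller.
; DamageObject applies environmental radial damage for physics on the world, plus direct damage of a configurable amount and type for health.
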(event EventDestroyed
  ;[1 1 1] Particle effect on destroyed
  (Effects|SpawnEmitteratLocation "/Game/StarterContent/Particles/P_Explosion.P_Explosion" (Transformation|GetActorLocation)))

(event Collision|EventActorBeginOverlap
  (params (OtherActor :type Actor%20Object%20Reference))
  ;[1 1 1] Damage actors (pawns) it overlaps
  (if (!= (Variables|/Script/Engine.Actor|GetInstigator OtherActor) self) ; Ignore your own projectiles
    (CallFunction|DamageObject OtherActor (Transformation|GetActorLocation))))

(event Collision|EventHit
  (params (MyComp :type Primitive%20Component%20Object%20Reference) (Other :type Actor%20Object%20Reference) (OtherComp :type Primitive%20Component%20Object%20Reference) (bSelfMoved :type Boolean) (HitLocation :type Vector) (HitNormal :type Vector) (NormalImpulse :type Vector :default "0, 0, 0") (Hit :type Hit%20Result%20Structure%20%28by%20ref%29))
  ;[1 1 1] Apply radial force and damage to hit object, then destroy projectile
  (CallFunction|DamageObject Other HitLocation))

(event EventBeginPlay)

(event EventActorBeginOverlap
  (params (OtherActor :type Actor%20Object%20Reference)))

(event EventTick
  (params (DeltaSeconds :type Float%20%28single-precision%29)))

(fn ConstructionScript)

(fn DamageObject
  (params (OtherActor :type Actor%20Object%20Reference) (HitLocation :type Vector))
  (bind _returnvalue (Game|GetInstigatorController))
  ;[1 1 1] Apply radial damage for physics vs world
  (if (!= (Game|GetInstigatorController OtherActor) _returnvalue)
    (Game|Damage|ApplyRadialDamage 1e+01 HitLocation (Variables|Default|GetDamageRadius) "/Engine/EngineDamageTypes/DmgTypeBP_Environmental.DmgTypeBP_Environmental_C" (Utilities|Array|MakeArray _returnvalue) self _returnvalue false "ECC_Visibility")
    ;[1 1 1] Apply damage for health purposes
    (Game|Damage|ApplyDamage OtherActor (Variables|Default|GetDamageAmount) (Game|GetInstigatorController) self "/Script/Engine.DamageType")
    (Actor|DestroyActor)))