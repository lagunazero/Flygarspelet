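; Enemy actor that steers toward a target actor, or a fixed location when none is set, and shoots at the target.
; Each tick it feeds the sign of yaw and pitch error to its movement component for bang-bang turning.
; Thrust scales with facing alignment, reversing within the slow-down distance while still moving forward.
; The shooting component fires when facing alignment with a valid target exceeds the fire-angle threshold.
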(event EventTick
  (params (DeltaSeconds :type Float%20%28single-precision%29))
  (bind _returnvalue (Transformation|GetActorRotation))
  (bind _returnvalue_2 (Transformation|GetActorLocation))
  (bind _movement_bp (Variables|Default|GetMovement_BP))
  ;[1 1 1] Use Actor's location or given TargetLocation?
  (|CallParentFunction DeltaSeconds)
  (bind _targettofollow (Variables|Default|GetTargetToFollow)
    (:then
      (Variables|Default|SetDesiredLocation (Transformation|GetActorLocation _targettofollow)))
    (:else
      (Variables|Default|SetDesiredLocation (Variables|Default|GetTargetLocation))))
  (Default|ApplyYaw _movement_bp (Math|Float|Sign(Float) (.Yaw (Math|Rotator|BreakRotator (Math|Rotator|Delta(Rotator) (Math|Rotator|FindLookatRotation _returnvalue_2 (Variables|Default|GetDesiredLocation)) _returnvalue)))))
  (Default|ApplyPitch _movement_bp (Math|Float|Sign(Float) (.Pitch (Math|Rotator|BreakRotator (Math|Rotator|Delta(Rotator) (Math|Rotator|FindLookatRotation _returnvalue_2 (Variables|Default|GetDesiredLocation)) _returnvalue)))))
  (Default|ApplyThrust _movement_bp (Math|Float|SelectFloat (Math|Float|SelectFloat -1.0 0.0 (>= (Variables|/Game/Blueprints/Components/Movement_BP.Movement_BP_C|GetCurrentForwardSpeed (Variables|Default|GetMovement_BP)) 5e+01)) (Math|Vector|DotProduct (Math|Vector|GetForwardVector (Math|Rotator|FindLookatRotation _returnvalue_2 (Variables|Default|GetDesiredLocation))) (Math|Vector|GetForwardVector _returnvalue)) (<= (Math|Vector|VectorLength (- _returnvalue_2 (Variables|Default|GetDesiredLocation))) (Variables|Default|GetSlowDownDistance)))) ; Use dot product of forward vectors to get "smooth" thrusting
  (Variables|Default|GetTargetToFollow
    (:then
      (if (> (Math|Vector|DotProduct (Math|Vector|GetForwardVector (Math|Rotator|FindLookatRotation _returnvalue_2 (Variables|Default|GetDesiredLocation))) (Math|Vector|GetForwardVector _returnvalue)) (Variables|Default|GetFireAngle))
        (Default|Shoot (Variables|Default|GetShooting_BP))))
    (:else)))

(fn ConstructionScript
  (|CallParentFunction))