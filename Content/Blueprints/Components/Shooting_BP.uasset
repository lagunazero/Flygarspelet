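; Shooting component that fires Projectile_BP actors from its owner, with a delay between shots.
; Tick counts the fire delay down to zero, and Shoot only fires at zero, then resets it to RateOfFire.
; Each shot spawns at the next emitter offset in a looping array, rotated with the owner, whose Pawn is set as instigator.
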(event EventBeginPlay)

(event EventTick
  (params (DeltaSeconds :type Float%20%28single-precision%29))
  ;[1 1 1] Reduce Fire delay
  (Variables|Default|SetCurrentFireDelay (Math|Float|Max(Float) (- (Variables|Default|GetCurrentFireDelay) DeltaSeconds) 0.0)))

(fn Shoot
  (bind _returnvalue (Components|GetOwner))
  ;[1 1 1] Shoot projectiles
  (if (<= (Variables|Default|GetCurrentFireDelay) 0.0)
    (bind _aspawn (Utilities|Casting|CastToPawn _returnvalue))
    (Game|SpawnActorfromClass "/Game/Blueprints/Actors/Projectile_BP.Projectile_BP_C" (Math|Transform|ComposeTransforms (Transformation|GetActorTransform _returnvalue) (Math|Conversions|ToTransform(Vector) (Math|Vector|RotateVector (Utilities|Array|Get(acopy) (Variables|Default|GetProjectileEmitterOffsets) (Variables|Default|GetCurrentProjectileEmitterIndex)) (Transformation|GetActorRotation _returnvalue)))) "Undefined" 0 _aspawn)
    ;[1 1 1] Increment Rate of Fire
    (Variables|Default|SetCurrentFireDelay (Variables|Default|GetRateOfFire))
    ;[1 1 1] Increment emitter index
    (if (< (+ (Variables|Default|GetCurrentProjectileEmitterIndex) 1) (Utilities|Array|Length (Variables|Default|GetProjectileEmitterOffsets)))
      (Math|Integer|IncrementInt (Variables|Default|GetCurrentProjectileEmitterIndex))
      (else
        (Variables|Default|SetCurrentProjectileEmitterIndex 0)))))