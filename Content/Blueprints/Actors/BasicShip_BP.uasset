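; BasicShip_BP is a ship actor that handles its own health, damage and kill credit.
; Construction sets Health to MaxHealth, and AnyDamage records unique instigating ships, then subtracts damage unless Invincible.
; Damage from a valid controller whose pawn is not a BasicShip_BP is ignored.
; Damage exceeding Health zeroes it, increments a valid instigator's KillCount, and sets AutoDestroyWhenFinished to defer destruction and block further damage.
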(event Game|Damage|EventAnyDamage
  (params (Damage :type Float%20%28single-precision%29) (DamageType :type Damage%20Type%20Object%20Reference) (InstigatedBy :type Controller%20Object%20Reference) (DamageCauser :type Actor%20Object%20Reference))
  (if (not (Variables|Default|GetbAutoDestroyWhenFinished))
    (Utilities|IsValid InstigatedBy
      (:Is%20Valid
        ;[1 1 1] Track damage instigators
        (Variables|Default|SetIsInstigatorValid true)
        (bind _asbasic_ship_bp (Utilities|Casting|CastToBasicShip_BP (Pawn|GetControlledPawn InstigatedBy)))
        (Utilities|Array|AddUnique (Variables|Default|GetDamageInstigators) _asbasic_ship_bp))
      (:Is%20Not%20Valid
        (Variables|Default|SetIsInstigatorValid false)))
    (if (not (Variables|Default|GetInvincible))
      (if (>= (- (Variables|Default|GetHealth) Damage) 0.0)
        ;[1 1 1] Injured
        (Variables|Default|SetHealth (- (Variables|Default|GetHealth) Damage))
        (else
          ;[1 1 1] Killed
          (Variables|Default|SetHealth 0.0)
          (if (Variables|Default|GetIsInstigatorValid)
            (Math|Integer|IncrementInt (Variables|BasicShip_BP_C|GetKillCount _asbasic_ship_bp)
              (:%20%20
                _)))
          (Variables|Default|SetbAutoDestroyWhenFinished true) ; Don't destroy immediately because that breaks references in other places. This takes a LONG time though
        )))))

(fn ConstructionScript
  (Variables|Default|SetHealth (Variables|Default|GetMaxHealth)))