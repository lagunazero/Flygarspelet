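; Spawner component that periodically creates AI pawns for the BasicShip_BP that owns it.
; A Tick countdown, first set to a fraction of its maximum on BeginPlay, calls SpawnActor and resets whenever it expires.
; SpawnActor spawns the configured class above the owner with matching rotation, then copies the owner's Faction if both are BasicShip_BP and prints a debug message.
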(event EventBeginPlay
  (Variables|Default|SetSpawnTimer (* (Variables|Default|GetSpawnTimerMax) (Variables|Default|GetSpawnTimeStartFaction))))

(event EventTick
  (params (DeltaSeconds :type Float%20%28single-precision%29))
  (Variables|Default|SetSpawnTimer (- (Variables|Default|GetSpawnTimer) DeltaSeconds))
  (if (<= (Variables|Default|GetSpawnTimer) 0.0)
    (Variables|Default|SetSpawnTimer (Variables|Default|GetSpawnTimerMax))
    (CallFunction|SpawnActor)))

(fn SpawnActor
  (bind _returnvalue (Components|GetOwner))
  (bind _returnvalue_2 (AI|SpawnAIFromClass (Variables|Default|GetSpawnActorType) 0 (+ (Transformation|GetActorLocation _returnvalue) "0, 0,200.000000") (Transformation|GetActorRotation _returnvalue) false))
  (bind _asbasic_ship_bp (Utilities|Casting|CastToBasicShip_BP (Components|GetOwner)))
  (bind _asbasic_ship_bp_2 (Utilities|Casting|CastToBasicShip_BP _returnvalue_2))
  (Variables|/Game/Blueprints/Actors/BasicShip_BP.BasicShip_BP_C|SetFaction _asbasic_ship_bp_2 (Variables|/Game/Blueprints/Actors/BasicShip_BP.BasicShip_BP_C|GetFaction _asbasic_ship_bp))
  (Development|PrintString (Utilities|String|Append (Utilities|GetDisplayName self) ": spawned actor " (Utilities|GetDisplayName _asbasic_ship_bp_2))))