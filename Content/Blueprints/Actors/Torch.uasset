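; Torch actor that makes its point light pulse smoothly between two colors.
; On BeginPlay it stores the light's current color as the start color and picks a random phase so torches can vary.
; Each Tick advances that phase by delta time and uses a sine remapped to 0–1 to lerp toward EndColor.
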(event EventBeginPlay
  (Variables|Default|SetStartColor (Rendering|Components|Light|GetLightColor (Variables|Default|GetPointLight)))
  (Variables|Default|SetLightGradient (Math|Random|RandomFloat)))

(event EventActorBeginOverlap
  (params (OtherActor :type Actor%20Object%20Reference)))

(event EventTick
  (params (DeltaSeconds :type Float%20%28single-precision%29))
  (Variables|Default|SetLightGradient (+ DeltaSeconds (Variables|Default|GetLightGradient)))
  (Rendering|Components|Light|SetLightColor (Variables|Default|GetPointLight) (Math|Color|Lerp(LinearColor) (Variables|Default|GetStartColor) (Variables|Default|GetEndColor) (/ (+ (Math|Trig|Sin(Radians) (+ DeltaSeconds (Variables|Default|GetLightGradient))) 1.0) 2.0)) true))

(fn ConstructionScript)